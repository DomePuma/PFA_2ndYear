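; Shared camera actor that frames all BP_Character actors in the level, gathered at BeginPlay, which also adds the sprint bar widget after a short delay.
; Each tick it moves to the targets' average position, with optional Z, blended toward player 0 by a distance-driven curve.
; When the first two targets are over 500 units apart, another curve sets spring arm length from their average distance to the camera actor.
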(event Custom|InitializeTargets
  (Utilities|Array|Clear (Variables|Default|GetTargets))
  (bind _outactors (Actor|GetAllActorsOfClass "/Game/Blueprint/BP_Character.BP_Character_C"))
  (Variables|Default|SetTargets _outactors))

(event Custom|AdjustLocation
  (Transformation|SetActorLocation (CallFunction|GetAdjustedLocation) false false))

(event Custom|AdjustCameraDistance
  (Variables|/Script/Engine.SpringArmComponent|SetTargetArmLength (Variables|Default|GetSpringArm) (CallFunction|GetAdjustedTargetSpringArmLength)))

(event EventBeginPlay
  (CallFunction|InitializeTargets)
  (Utilities|FlowControl|Delay 0.1)
  (bind _returnvalue (UserInterface|CreateWidget "/Game/Widget/W_Sprint_bar.W_Sprint_bar_C"))
  (UserInterface|Viewport|AddtoViewport _returnvalue 0))

(event EventTick
  (params (DeltaSeconds :type Float%20%28single-precision%29))
  (bind _targets (Variables|Default|GetTargets))
  (CallFunction|AdjustLocation)
  (if (> (Transformation|GetDistanceTo (Utilities|Array|Get(acopy) _targets) (Utilities|Array|Get(acopy) _targets 1)) 5e+02)
    (CallFunction|AdjustCameraDistance)))

(fn ConstructionScript)

(fn GetAdjustedLocation
  (return (Math|Vector|Lerp(Vector) (CallFunction|GetCenterPoint) (Transformation|GetActorLocation (Game|GetPlayerCharacter 0)) (Math|Curves|GetFloatValue (Variables|Default|GetC_LocationAlpha) (Math|Vector|Distance(Vector) (CallFunction|GetCenterPoint) (Transformation|GetActorLocation (Game|GetPlayerCharacter 0)))))))

(fn GetCenterPoint
  (for _array_element (Variables|Default|GetTargets)
    (bind _output_get (LocalVariables|SetVector%20Sum (+ (LocalVariables|GetVector%20Sum) (Transformation|GetActorLocation _array_element)))))
  (bind _output_get_2 (Variables|Default|SetCenterPoint (/ _output_get (Utilities|Array|Length (Variables|Default|GetTargets)))))
  (return (Math|Vector|MakeVector (.x _output_get_2) (.y _output_get_2) (Math|Float|SelectFloat (.z _output_get_2) 0.0 (Variables|Default|GetTakeZValue)))))

(fn GetAdjustedTargetSpringArmLength
  (for _array_element (Variables|Default|GetTargets)
    (LocalVariables|SetTotalDistance (+ (LocalVariables|GetTotalDistance) (Math|Vector|VectorLength (- (Transformation|GetActorLocation _array_element) (Transformation|GetActorLocation))))))
  (return (Math|Curves|GetFloatValue (Variables|Default|GetC_CamDistance) (/ (LocalVariables|GetTotalDistance) (Utilities|Array|Length (Variables|Default|GetTargets))))))