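; Fire character Blueprint that lets the player shoot fireballs and interact with buttons, incubators and portable boxes.
; Interact branches on the overlapped object's type, attaching boxes to the right-hand socket with brief movement locks and a grab cooldown.
; Held boxes drop only when a downward hand trace hits within a distance range.
; Tick resets control rotation, clears interaction state and refills the time-based gauge that gates grounded fireball shots.
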(event OnComponentEndOverlap(InteractionBox)
  (params (OverlappedComponent :type Primitive%20Component%20Object%20Reference) (OtherActor :type Actor%20Object%20Reference) (OtherComp :type Primitive%20Component%20Object%20Reference) (OtherBodyIndex :type Integer))
  (Variables|Default|SetInteractableObjectRef 0))

(event Custom|Cooldown
  (Utilities|FlowControl|Delay (Variables|Default|GetCooldownGrab))
  (Variables|Default|SetCanGrab true))

(event Custom|RemoveBox
  (Variables|Default|SetIsHoldingBox false)
  (Variables|Default|SetCanGrab false)
  (Utilities|FlowControl|Delay 0.4)
  (Class|BPIInteractableObject|DesactivateInteraction(Message) (Variables|Default|GetBoxHold))
  (Transformation|DetachFromActor (Variables|Default|GetBoxHold) "KeepWorld" "KeepWorld" "KeepWorld")
  (Variables|Default|SetCanMove true)
  (Variables|Default|SetBoxHold 0)
  (CallFunction|Cooldown))

(event EventTick
  (params (DeltaSeconds :type Float%20%28single-precision%29))
  (CallFunction|RotationReset)
  (CallFunction|CheckInteraction)
  (CallFunction|ReloadFireGauge))

(event Input|ActionEvents|InputActionSprint/FireBall
  (params (Key :type Key%20Structure :default "None"))
  (:Pressed
    (if (not (AI|Components|NavMovement|IsFalling (Variables|Character|GetCharacterMovement)))
      (if (>= (Variables|Default|GetFireGauge) (Variables|Default|GetCooldownFire))
        (Variables|Default|SetIsShooting true)
        (Audio|PlaySoundatLocation "/Game/Audio/Sounds/Fire_ball.Fire_ball" (Transformation|GetWorldLocation (Variables|Character|GetMesh)) "0, 0, 0" 1.0 1.0 0.0 0 0 0 0)
        (Utilities|FlowControl|Delay 0.2)
        (Variables|Default|SetIsShooting false)
        (Game|SpawnActorfromClass "/Game/Blueprint/BP_FireBall.BP_FireBall_C" (Math|Transform|MakeTransform (Transformation|GetWorldLocation (Variables|Default|GetSphere_0)) (Transformation|GetActorRotation)) "AlwaysSpawn" 0 0)
        (Variables|Default|SetFireGauge 0.0)))))

(event Input|ActionEvents|InputActionInteractElectric
  (params (Key :type Key%20Structure :default "None"))
  (bind _mesh (Variables|Character|GetMesh))
  (bind _interactionbox (Variables|Default|GetInteractionBox))
  (bind _overlappingactors (Collision|GetOverlappingActors _interactionbox "/Game/Blueprint/BP_InteractableObject.BP_InteractableObject_C" :!class /Script/Engine.PrimitiveComponent))
  (bind _returnvalue (Transformation|GetSocketLocation _mesh "RightHandBoneSocket"))
  (bind _output (Utilities|Array|Get(acopy) _overlappingactors))
  (:Pressed
    (if (Variables|Default|GetCanGrab)
      (if (== (.z (Variables|/Script/Engine.MovementComponent|GetVelocity (Variables|Character|GetCharacterMovement))) 0.0)
        (if (Variables|Default|GetIsHoldingBox)
          (bind _outhit (Collision|LineTraceForObjects _returnvalue (+ _returnvalue (* (Math|Vector|VectorDown) 1e+03)) (Variables|Default|GetObjectTypeRaycastHit) false 0 "None"))
          (if (and (< (.distance _outhit) (Variables|Default|GetMaxDistance)) (> (.distance _outhit) (Variables|Default|GetMinDistance)))
            (Variables|Default|SetCanMove false)
            (Variables|Default|SetIsHoldingBox false)
            (Variables|Default|SetCanGrab false)
            (Utilities|FlowControl|Delay 0.4)
            (Class|BPIInteractableObject|DesactivateInteraction(Message) (Variables|Default|GetBoxHold))
            (Transformation|DetachFromActor (Variables|Default|GetBoxHold) "KeepWorld" "KeepWorld" "KeepWorld")
            (Variables|Default|SetCanMove true)
            (Variables|Default|SetBoxHold 0)
            (CallFunction|Cooldown))
          (elif (Collision|IsOverlappingActor _interactionbox _output :!class /Script/Engine.PrimitiveComponent)
            (Variables|Default|SetInteractableObjectRef _output)
            (bind _asbp_interactable_object (Utilities|Casting|CastToBP_InteractableObject _output))
            (switch Utilities|FlowControl|Switch|SwitchonE_InteractableButtonType (Variables|/Game/Blueprint/BP_InteractableObject.BP_InteractableObject_C|GetObjectType _asbp_interactable_object)
              (:NewEnumerator0
                (Default|ActivateInteraction _asbp_interactable_object))
              (:NewEnumerator2
                (Variables|Default|SetCanMove false)
                (Audio|PlaySoundatLocation "/Game/Audio/Sounds/Lift_kcp.Lift_kcp" (Transformation|GetWorldLocation (Variables|Character|GetMesh)) "0, 0, 0" 1.0 1.0 0.0 0 0 0 0)
                (bind _asbp_portable_pressure_plate_box (Utilities|Casting|CastToBP_PortablePressurePlateBox (Variables|Default|GetInteractableObjectRef))
                  (:then
                    (if (not (Variables|/Game/Blueprint/BP_PortablePressurePlateBox.BP_PortablePressurePlateBox_C|GetIsPlaced _asbp_portable_pressure_plate_box))
                      (if (not (Variables|/Game/Blueprint/BP_PortablePressurePlateBox.BP_PortablePressurePlateBox_C|GetIsOnBox _asbp_portable_pressure_plate_box))
                        (bind _output_get (Variables|Default|SetBoxHold (Variables|Default|GetInteractableObjectRef)))
                        (Transformation|AttachComponentToComponent _output_get (Variables|Character|GetMesh) "RightHandBoneSocket" "SnapToTarget" "SnapToTarget" "KeepWorld" false)
                        (Variables|Default|SetCanGrab false)
                        (Variables|Default|SetIsHoldingBox true)
                        (CallFunction|Cooldown)
                        (Default|ActivateInteraction _asbp_portable_pressure_plate_box)
                        (Utilities|FlowControl|Delay 0.5 :!label _label)
                        (Variables|Default|SetCanMove true))))
                  (:CastFailed
                    (bind _asbp_portable_big_box (Utilities|Casting|CastToBP_PortableBigBox (Variables|Default|GetInteractableObjectRef))
                      (:then
                        (if (not (Variables|/Game/Blueprint/BP_PortableBigBox.BP_PortableBigBox_C|GetIsPlaced _asbp_portable_big_box))
                          (if (not (Variables|/Game/Blueprint/BP_PortableBigBox.BP_PortableBigBox_C|GetIsOnBox _asbp_portable_big_box))
                            (Development|PrintString "1")
                            (bind _output_get_2 (Variables|Default|SetBoxHold (Variables|Default|GetInteractableObjectRef)))
                            (Transformation|AttachComponentToComponent _output_get_2 (Variables|Character|GetMesh) "RightHandBoneSocket" "SnapToTarget" "SnapToTarget" "KeepWorld" false)
                            (Variables|Default|SetCanGrab false)
                            (Variables|Default|SetIsHoldingBox true)
                            (CallFunction|Cooldown)
                            (Default|ActivateInteraction _asbp_portable_big_box)
                            (goto _label))))
                      (:CastFailed
                        (bind _asbp_portable_platform_box (Utilities|Casting|CastToBP_PortablePlatformBox (Variables|Default|GetInteractableObjectRef)))
                        (if (not (Variables|/Game/Blueprint/BP_PortablePlatformBox.BP_PortablePlatformBox_C|GetIsPlaced _asbp_portable_platform_box))
                          (if (not (Variables|/Game/Blueprint/BP_PortablePlatformBox.BP_PortablePlatformBox_C|GetIsOnBox _asbp_portable_platform_box))
                            (bind _output_get_3 (Variables|Default|SetBoxHold (Variables|Default|GetInteractableObjectRef)))
                            (Transformation|AttachComponentToComponent _output_get_3 (Variables|Character|GetMesh) "RightHandBoneSocket" "SnapToTarget" "SnapToTarget" "KeepWorld" false)
                            (Variables|Default|SetCanGrab false)
                            (Variables|Default|SetIsHoldingBox true)
                            (CallFunction|Cooldown)
                            (Default|ActivateInteraction _asbp_portable_platform_box)
                            (goto _label))))))))
              (:NewEnumerator5
                (bind _asbp_incubator (Utilities|Casting|CastToBP_Incubator _asbp_interactable_object))
                (Default|ChangeLevel _asbp_incubator)))))))))

(fn ConstructionScript
  (|CallParentFunction))

(fn RotationReset
  (Pawn|SetControlRotation (Pawn|GetController) (Math|Rotator|MakeRotator 0.0 0.0 0.0)))

(fn CheckInteraction
  (if (<= (.z (Variables|/Script/Engine.MovementComponent|GetVelocity (Variables|Character|GetCharacterMovement))) 0.0)
    (Variables|Default|SetIsInteracting false)))

(fn ReloadFireGauge
  (if (< (Variables|Default|GetFireGauge) (Variables|Default|GetCooldownFire))
    (Variables|Default|SetFireGauge (+ (Variables|Default|GetFireGauge) (Utilities|Time|GetWorldDeltaSeconds)))))