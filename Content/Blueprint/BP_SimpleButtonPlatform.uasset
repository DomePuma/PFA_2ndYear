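; Button-activated moving platform that, once triggered by ActivateInteraction, shuttles back and forth indefinitely.
; BeginPlay hides the prompt widget and derives the end position from the Door component's world location plus per-axis move offsets.
; A timeline lerps Door between both points, with a FlipFlop alternating reverse and play after a short delay at each end.
; Sphere overlap shows the interaction prompt only before activation.
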(event OnComponentBeginOverlap(Sphere)
  (params (OverlappedComponent :type Primitive%20Component%20Object%20Reference) (OtherActor :type Actor%20Object%20Reference) (OtherComp :type Primitive%20Component%20Object%20Reference) (OtherBodyIndex :type Integer) (bFromSweep :type Boolean) (SweepResult :type Hit%20Result%20Structure%20%28by%20ref%29))
  ;[1 1 1] Interact_prompt
  (if (not (Variables|Default|GetIsActivated))
    (Rendering|SetVisibility (Variables|Default|GetWidget) true false)))

(event OnComponentEndOverlap(Sphere)
  (params (OverlappedComponent :type Primitive%20Component%20Object%20Reference) (OtherActor :type Actor%20Object%20Reference) (OtherComp :type Primitive%20Component%20Object%20Reference) (OtherBodyIndex :type Integer))
  ;[1 1 1] Interact_prompt
  (Rendering|SetVisibility (Variables|Default|GetWidget) false false))

(event EventBeginPlay
  (Rendering|SetVisibility (Variables|Default|GetWidget) false false)
  (Variables|Default|SetBaseLocation (Transformation|GetWorldLocation (Variables|Default|GetDoor)))
  (Variables|Default|SetEndLocation (Math|Vector|MakeVector (+ (.x (Variables|Default|GetBaseLocation)) (Variables|Default|GetMoveXValue)) (+ (.y (Variables|Default|GetBaseLocation)) (Variables|Default|GetMoveYValue)) (+ (.z (Variables|Default|GetBaseLocation)) (Variables|Default|GetMoveZValue)))))

(event EventActivateInteraction
  (Variables|Default|SetIsActivated true)
  (bind _newtrack_0 (Timeline|OpenDoor Play)
    (:Update
      (Transformation|SetWorldLocation (Variables|Default|GetDoor) (Math|Vector|Lerp(Vector) (Variables|Default|GetBaseLocation) (Variables|Default|GetEndLocation) _newtrack_0) false false))
    (:Finished
      (Utilities|FlowControl|Delay 1.0)
      (Utilities|FlowControl|FlipFlop
        (:A
          (Timeline|OpenDoor Reverse))
        (:B
          (Timeline|OpenDoor Play))))))

(fn ConstructionScript)