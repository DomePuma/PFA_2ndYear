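; BP_SimpleButtonDoor is a button-operated door that moves when interacted with.
; An overlap sphere shows and hides the interact prompt widget.
; ActivateInteraction plays sounds at the button and door, then runs a timeline lerping the door toward its BeginPlay location plus configurable XYZ offsets.
; The lerp starts from the door's current location each update, so motion compounds rather than following the curve directly; no closing logic exists.
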(event OnComponentBeginOverlap(Sphere)
  (params (OverlappedComponent :type Primitive%20Component%20Object%20Reference) (OtherActor :type Actor%20Object%20Reference) (OtherComp :type Primitive%20Component%20Object%20Reference) (OtherBodyIndex :type Integer) (bFromSweep :type Boolean) (SweepResult :type Hit%20Result%20Structure%20%28by%20ref%29))
  ;[1 1 1] Interact_prompt
  (Rendering|SetVisibility (Variables|Default|GetWidget) true false))

(event OnComponentEndOverlap(Sphere)
  (params (OverlappedComponent :type Primitive%20Component%20Object%20Reference) (OtherActor :type Actor%20Object%20Reference) (OtherComp :type Primitive%20Component%20Object%20Reference) (OtherBodyIndex :type Integer))
  ;[1 1 1] Interact_prompt
  (Rendering|SetVisibility (Variables|Default|GetWidget) false false))

(event EventBeginPlay
  (Rendering|SetVisibility (Variables|Default|GetWidget) false false)
  (Variables|Default|SetBaseLocation (Transformation|GetWorldLocation (Variables|Default|GetDoor))))

(event EventActivateInteraction
  (bind _baselocation (Variables|Default|GetBaseLocation))
  (Audio|PlaySoundatLocation "/Game/Audio/Sounds/générator_activation.générator_activation" (Transformation|GetWorldLocation (Variables|Default|GetButton)) "0, 0, 0" 1.0 1.0 0.0 0 0 0 0)
  (Audio|PlaySoundatLocation (Variables|Default|GetSoundToPlay) (Transformation|GetWorldLocation (Variables|Default|GetDoor)) "0, 0, 0" 1.0 1.0 0.0 0 0 0 0)
  (bind _newtrack_0 (Timeline|OpenDoor Play)
    (:Update
      (Transformation|SetWorldLocation (Variables|Default|GetDoor) (Math|Vector|Lerp(Vector) (Transformation|GetWorldLocation (Variables|Default|GetDoor)) (Math|Vector|MakeVector (+ (.x _baselocation) (Variables|Default|GetMoveXValue)) (+ (.y _baselocation) (Variables|Default|GetMoveYValue)) (+ (.z _baselocation) (Variables|Default|GetMoveZValue))) _newtrack_0) false false))))

(fn ConstructionScript)