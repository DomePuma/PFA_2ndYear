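; Portable pressure plate box that tracks whether it is held or placed and shows an interact prompt for the fire character.
; Interaction events toggle the held state, and activation also marks the box as placed when it cannot be re-picked.
; The sphere overlap shows the widget only when the box is neither held, placed nor on a box.
; Hits against anything except characters and other portable boxes stop the cube's physics.
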(event OnComponentBeginOverlap(Sphere)
  (params (OverlappedComponent :type Primitive%20Component%20Object%20Reference) (OtherActor :type Actor%20Object%20Reference) (OtherComp :type Primitive%20Component%20Object%20Reference) (OtherBodyIndex :type Integer) (bFromSweep :type Boolean) (SweepResult :type Hit%20Result%20Structure%20%28by%20ref%29))
  ;[1 1 1] Interact_Prompt
  (Utilities|Casting|CastToBP_FireCharacter_2 OtherActor)
  (if (not (Variables|Default|GetIsOnBox))
    (if (not (Variables|Default|GetIsHold))
      (if (not (Variables|Default|GetIsPlaced))
        (Rendering|SetVisibility (Variables|Default|GetWidget) true false)))))

(event OnComponentEndOverlap(Sphere)
  (params (OverlappedComponent :type Primitive%20Component%20Object%20Reference) (OtherActor :type Actor%20Object%20Reference) (OtherComp :type Primitive%20Component%20Object%20Reference) (OtherBodyIndex :type Integer))
  ;[1 1 1] Interact_Prompt
  (Utilities|Casting|CastToBP_FireCharacter_2 OtherActor)
  (Rendering|SetVisibility (Variables|Default|GetWidget) false false))

(event Custom|StopSimulatePhysics
  (Physics|SetSimulatePhysics (Variables|Default|GetCube) false))

(event EventActivateInteraction
  (Variables|Default|SetIsHold true)
  (if (not (Variables|Default|GetCanBeRepicked))
    (Variables|Default|SetIsPlaced true)))

(event Collision|EventHit
  (params (MyComp :type Primitive%20Component%20Object%20Reference) (Other :type Actor%20Object%20Reference) (OtherComp :type Primitive%20Component%20Object%20Reference) (bSelfMoved :type Boolean) (HitLocation :type Vector :default "0, 0, 0") (HitNormal :type Vector :default "0, 0, 0") (NormalImpulse :type Vector :default "0, 0, 0") (Hit :type Hit%20Result%20Structure%20%28by%20ref%29))
  (Utilities|Casting|CastToBP_Character Other
    (:CastFailed
      (Utilities|Casting|CastToBP_PortablePressurePlateBox Other
        (:CastFailed
          (Utilities|Casting|CastToBP_PortableBigBox Other
            (:CastFailed
              (Utilities|Casting|CastToBP_PortablePlatformBox Other
                (:CastFailed
                  (CallFunction|StopSimulatePhysics))))))))))

(event EventBeginPlay
  ;[1 1 1] Interact_Prompt
  (Rendering|SetVisibility (Variables|Default|GetWidget) false false))

(event EventDesactivateInteraction
  (Variables|Default|SetIsHold false))

(fn ConstructionScript
  (|CallParentFunction))