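; Electric character Blueprint that lets the player operate button-driven doors and platforms through its own Interact Electric input.
; On press, it stores the first interactable overlapping its InteractionBox and, for Hold Button types, casts to hold-button door, simple-button door or platform to activate it.
; Releasing while overlapping, or any end overlap on the box, deactivates the stored object and closes hold-button doors.
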(event OnComponentEndOverlap(InteractionBox)
  (params (OverlappedComponent :type Primitive%20Component%20Object%20Reference) (OtherActor :type Actor%20Object%20Reference) (OtherComp :type Primitive%20Component%20Object%20Reference) (OtherBodyIndex :type Integer))
  (bind _asbp_interactable_object (Utilities|Casting|CastToBP_InteractableObject (Variables|Default|GetInteractableObjectRef)))
  (Default|DesactivateInteraction _asbp_interactable_object)
  (switch Utilities|FlowControl|Switch|SwitchonE_InteractableButtonType (Variables|/Game/Blueprint/BP_InteractableObject.BP_InteractableObject_C|GetObjectType _asbp_interactable_object)
    (:NewEnumerator1
      (bind _asbp_hold_button_door (Utilities|Casting|CastToBP_HoldButtonDoor _asbp_interactable_object))
      (Default|CloseDoor _asbp_hold_button_door)
      (Variables|Default|SetInteractableObjectRef 0))))

(event Input|ActionEvents|InputActionInteractElectric
  (params (Key :type Key%20Structure))
  (bind _interactionbox (Variables|Default|GetInteractionBox))
  (bind _overlappingactors (Collision|GetOverlappingActors _interactionbox "/Game/Blueprint/BP_InteractableObject.BP_InteractableObject_C" :!class /Script/Engine.PrimitiveComponent))
  (bind _output (Utilities|Array|Get(acopy) _overlappingactors))
  (bind _returnvalue (Collision|IsOverlappingActor _interactionbox _output :!class /Script/Engine.PrimitiveComponent))
  (:Pressed
    (if _returnvalue
      (Variables|Default|SetInteractableObjectRef _output)
      (bind _asbp_interactable_object (Utilities|Casting|CastToBP_InteractableObject _output))
      (switch Utilities|FlowControl|Switch|SwitchonE_InteractableButtonType (Variables|/Game/Blueprint/BP_InteractableObject.BP_InteractableObject_C|GetObjectType _asbp_interactable_object)
        (:NewEnumerator1
          (bind _asbp_hold_button_door (Utilities|Casting|CastToBP_HoldButtonDoor _asbp_interactable_object)
            (:then
              (Default|ActivateInteraction _asbp_hold_button_door)
              (Default|OpenDoor _asbp_hold_button_door))
            (:CastFailed
              (bind _asbp_simple_button_door (Utilities|Casting|CastToBP_SimpleButtonDoor _asbp_interactable_object)
                (:then
                  (Default|ActivateInteraction _asbp_simple_button_door))
                (:CastFailed
                  (bind _asbp_simple_button_platform (Utilities|Casting|CastToBP_SimpleButtonPlatform _asbp_interactable_object))
                  (Default|ActivateInteraction _asbp_simple_button_platform)))))))))
  (:Released
    (if _returnvalue
      (bind _asbp_interactable_object_2 (Utilities|Casting|CastToBP_InteractableObject (Variables|Default|GetInteractableObjectRef)))
      (Default|DesactivateInteraction _asbp_interactable_object_2)
      (switch Utilities|FlowControl|Switch|SwitchonE_InteractableButtonType (Variables|/Game/Blueprint/BP_InteractableObject.BP_InteractableObject_C|GetObjectType _asbp_interactable_object_2)
        (:NewEnumerator1
          (bind _asbp_hold_button_door_2 (Utilities|Casting|CastToBP_HoldButtonDoor _asbp_interactable_object_2))
          (Default|CloseDoor _asbp_hold_button_door_2)
          (Variables|Default|SetInteractableObjectRef 0))))))

(fn ConstructionScript
  (|CallParentFunction))