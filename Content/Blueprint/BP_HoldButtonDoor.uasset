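; Sliding door actor, named as a hold-button door, that moves open or closed through externally triggered events.
; Separate open and close timelines lerp the door from its current location toward an offset or its BeginPlay position, alongside audio triggers.
; ActivateInteraction stops the closing timeline and DesactivateInteraction stops the opening one.
; A sphere overlap with BP_ElectricCharacter_2 toggles the prompt widget, which also hides on open and reappears on close.
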(event OnComponentBeginOverlap(Sphere)
  (params (OverlappedComponent :type Primitive%20Component%20Object%20Reference) (OtherActor :type Actor%20Object%20Reference) (OtherComp :type Primitive%20Component%20Object%20Reference) (OtherBodyIndex :type Integer) (bFromSweep :type Boolean) (SweepResult :type Hit%20Result%20Structure%20%28by%20ref%29))
  ;[1 1 1] Interact_prompt
  (Utilities|Casting|CastToBP_ElectricCharacter_2 OtherActor)
  (Rendering|SetVisibility (Variables|Default|GetWidget) true false))

(event OnComponentEndOverlap(Sphere)
  (params (OverlappedComponent :type Primitive%20Component%20Object%20Reference) (OtherActor :type Actor%20Object%20Reference) (OtherComp :type Primitive%20Component%20Object%20Reference) (OtherBodyIndex :type Integer))
  ;[1 1 1] Interact_prompt
  (Utilities|Casting|CastToBP_ElectricCharacter_2 OtherActor)
  (Rendering|SetVisibility (Variables|Default|GetWidget) false false))

(event Custom|CloseDoor
  (Class|AudioParameterControllerInterface|SetTriggerParameter (Variables|Default|GetAudio) "OnStop")
  (Variables|Default|SetIsOpenning false)
  (Rendering|SetVisibility (Variables|Default|GetWidget) true false)
  (bind _newtrack_0 (Timeline|CloseDoorTimeline PlayFromStart)
    (:Update
      (Transformation|SetWorldLocation (Variables|Default|GetDoor) (Math|Vector|Lerp(Vector) (Transformation|GetWorldLocation (Variables|Default|GetDoor)) (stale EventBeginPlay _output_get) _newtrack_0) false false))))

(event Custom|OpenDoor
  (bind _baselocation (Variables|Default|GetBaseLocation))
  (Class|AudioParameterControllerInterface|SetTriggerParameter (Variables|Default|GetAudio) "OnPlay")
  (Class|AudioParameterControllerInterface|SetTriggerParameter (Variables|Default|GetElectricPlatformSound) "OnPlay")
  (Variables|Default|SetIsOpenning true)
  (Rendering|SetVisibility (Variables|Default|GetWidget) false false)
  (bind _newtrack_0 (Timeline|OpenDoorTimeline PlayFromStart)
    (:Update
      (Transformation|SetWorldLocation (Variables|Default|GetDoor) (Math|Vector|Lerp(Vector) (Transformation|GetWorldLocation (Variables|Default|GetDoor)) (Math|Vector|MakeVector (+ (.x _baselocation) (Variables|Default|GetMoveXValue)) (+ (.y _baselocation) (Variables|Default|GetMoveYValue)) (+ (.z _baselocation) (Variables|Default|GetMoveZValue))) _newtrack_0) false false))))

(event EventBeginPlay
  (Rendering|SetVisibility (Variables|Default|GetWidget) false false)
  (bind _output_get (Variables|Default|SetBaseLocation (Transformation|GetWorldLocation (Variables|Default|GetDoor)))))

(event EventActivateInteraction
  (bind _newtrack_0 (Timeline|CloseDoorTimeline Stop)
    (:Update
      (Transformation|SetWorldLocation (Variables|Default|GetDoor) (Math|Vector|Lerp(Vector) (Transformation|GetWorldLocation (Variables|Default|GetDoor)) (stale EventBeginPlay _output_get) _newtrack_0) false false))))

(event EventDesactivateInteraction
  (bind _baselocation (Variables|Default|GetBaseLocation))
  (bind _newtrack_0 (Timeline|OpenDoorTimeline Stop)
    (:Update
      (Transformation|SetWorldLocation (Variables|Default|GetDoor) (Math|Vector|Lerp(Vector) (Transformation|GetWorldLocation (Variables|Default|GetDoor)) (Math|Vector|MakeVector (+ (.x _baselocation) (Variables|Default|GetMoveXValue)) (+ (.y _baselocation) (Variables|Default|GetMoveYValue)) (+ (.z _baselocation) (Variables|Default|GetMoveZValue))) _newtrack_0) false false))))

(fn ConstructionScript)