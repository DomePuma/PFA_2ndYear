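; Portable platform box that tracks whether it is held, placed or occupied by the Electric character.
; Interaction events toggle the held state, and non-repickable boxes are marked placed on activation.
; Sphere overlap shows the Fire character a prompt only when the box is free, while Tick polls Box overlap for the Electric character.
; Hits from anything but characters or portable boxes switch off physics simulation.
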(event OnComponentBeginOverlap(Sphere)
  (params (OverlappedComponent :type Primitive%20Component%20Object%20Reference) (OtherActor :type Actor%20Object%20Reference) (OtherComp :type Primitive%20Component%20Object%20Reference) (OtherBodyIndex :type Integer) (bFromSweep :type Boolean) (SweepResult :type Hit%20Result%20Structure%20%28by%20ref%29))
  ;[1 1 1] Interact_Prompt
  (Utilities|Casting|CastToBP_FireCharacter_2 OtherActor)
  (if (not (Variables|Default|GetIsOnBox))
    (if (not (Variables|Default|GetIsHold))
      (if (not (Variables|Default|GetIsPlaced))
        (Rendering|SetVisibility (Variables|Default|GetWidget) true false)))))

(event OnComponentEndOverlap(Sphere)
  (params (OverlappedComponent :type Primitive%20Component%20Object%20Reference) (OtherActor :type Actor%20Object%20Reference) (OtherComp :type Primitive%20Component%20Object%20Reference) (OtherBodyIndex :type Integer))
  ;[1 1 1] Interact_Prompt
  (Utilities|Casting|CastToBP_FireCharacter_2 OtherActor)
  (Rendering|SetVisibility (Variables|Default|GetWidget) false false))

(event OnComponentHit(Cube)
  (params (HitComponent :type Primitive%20Component%20Object%20Reference) (OtherActor :type Actor%20Object%20Reference) (OtherComp :type Primitive%20Component%20Object%20Reference) (NormalImpulse :type Vector :default "0, 0, 0") (Hit :type Hit%20Result%20Structure%20%28by%20ref%29))
  (bind _asbp_character (Utilities|Casting|CastToBP_Character OtherActor)
    (:then
      (Utilities|Casting|CastToBP_ElectricCharacter_2 _asbp_character)
      (Variables|Default|SetIsOnBox false))
    (:CastFailed
      (Utilities|Casting|CastToBP_PortablePressurePlateBox OtherActor
        (:CastFailed
          (Utilities|Casting|CastToBP_PortableBigBox OtherActor
            (:CastFailed
              (Utilities|Casting|CastToBP_PortablePlatformBox OtherActor
                (:CastFailed
                  (CallFunction|StopSimulatePhysics))))))))))

(event Custom|StopSimulatePhysics
  (Physics|SetSimulatePhysics (Variables|Default|GetCube) false))

(event EventActivateInteraction
  (Variables|Default|SetIsHold true)
  (if (not (Variables|Default|GetCanBeRepicked))
    (Variables|Default|SetIsPlaced true)))

(event EventBeginPlay
  ;[1 1 1] Interact_Prompt
  (Rendering|SetVisibility (Variables|Default|GetWidget) false false))

(event EventTick
  (params (DeltaSeconds :type Float%20%28single-precision%29))
  (if (Collision|IsOverlappingActor (Variables|Default|GetBox) (Utilities|Array|Get(acopy) (Collision|GetOverlappingActors (Variables|Default|GetBox) "/Game/Blueprint/BP_ElectricCharacter_2.BP_ElectricCharacter_2_C" :!class /Script/Engine.PrimitiveComponent)) :!class /Script/Engine.PrimitiveComponent)
    (Variables|Default|SetIsOnBox true)
    (else
      (Variables|Default|SetIsOnBox false))))

(event EventDesactivateInteraction
  (Variables|Default|SetIsHold false))

(fn ConstructionScript
  (|CallParentFunction))