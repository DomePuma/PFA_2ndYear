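; BP_FireCharacter is a character Blueprint that lets the player press simple buttons and carry portable boxes.
; The Interact Electric input drops any held box; otherwise it takes the first BP_InteractableObject overlapping InteractionBox and branches on ObjectType.
; Boxes attach to the Sphere component and toggle their interaction message on pickup and drop.
; An older PhysicsConstraint-based carry for BP_PortablePressurePlateBox remains as disabled, unreachable nodes.
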(event OnComponentEndOverlap(InteractionBox)
  (params (OverlappedComponent :type Primitive%20Component%20Object%20Reference) (OtherActor :type Actor%20Object%20Reference) (OtherComp :type Primitive%20Component%20Object%20Reference) (OtherBodyIndex :type Integer))
  (Variables|Default|SetInteractableObjectRef 0))

(event Input|ActionEvents|InputActionInteractElectric
  (params (Key :type Key%20Structure))
  (bind _interactionbox (Variables|Default|GetInteractionBox))
  (bind _overlappingactors (Collision|GetOverlappingActors _interactionbox "/Game/Blueprint/BP_InteractableObject.BP_InteractableObject_C" :!class /Script/Engine.PrimitiveComponent))
  (bind _output (Utilities|Array|Get(acopy) _overlappingactors))
  (:Pressed
    (if (Variables|Default|GetIsHoldingBox)
      (Transformation|DetachFromActor (Variables|Default|GetBoxHold) "KeepWorld" "KeepWorld" "KeepWorld")
      (Variables|Default|SetIsHoldingBox false)
      (Class|BPIInteractableObject|DesactivateInteraction(Message) (Variables|Default|GetBoxHold))
      (Variables|Default|SetBoxHold 0)
      (elif (Collision|IsOverlappingActor _interactionbox _output :!class /Script/Engine.PrimitiveComponent)
        (Variables|Default|SetInteractableObjectRef _output)
        (bind _asbp_interactable_object (Utilities|Casting|CastToBP_InteractableObject _output))
        (switch Utilities|FlowControl|Switch|SwitchonE_InteractableButtonType (Variables|/Game/Blueprint/BP_InteractableObject.BP_InteractableObject_C|GetObjectType _asbp_interactable_object)
          (:NewEnumerator0
            (Default|ActivateInteraction _asbp_interactable_object))
          (:NewEnumerator2
            (bind _output_get (Variables|Default|SetBoxHold (Variables|Default|GetInteractableObjectRef)))
            (Class|BPIInteractableObject|ActivateInteraction(Message) _output_get)
            (Transformation|AttachComponentToComponent (Variables|Default|GetInteractableObjectRef) (Variables|Default|GetSphere) "None" "SnapToTarget" "KeepWorld" "KeepWorld" false)
            (Variables|Default|SetIsHoldingBox true)))))))

(fn ConstructionScript
  (|CallParentFunction))