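; Fire-activated platform that moves its Door component when a BP_FireBall hits its Button component.
; On BeginPlay it caches the Door's world location and adds the X, Y and Z move values to get the end point.
; A fireball hit plays the OpenDoor timeline, which lerps the Door between those points.
; The FlipFlop toggle is disabled, so nothing reverses the movement.
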(event OnComponentHit(Button)
  (params (HitComponent :type Primitive%20Component%20Object%20Reference) (OtherActor :type Actor%20Object%20Reference) (OtherComp :type Primitive%20Component%20Object%20Reference) (NormalImpulse :type Vector :default "0, 0, 0") (Hit :type Hit%20Result%20Structure%20%28by%20ref%29))
  (Utilities|Casting|CastToBP_FireBall OtherActor)
  (bind _newtrack_0 (Timeline|OpenDoor Play)
    (:Update
      (Transformation|SetWorldLocation (Variables|Default|GetDoor) (Math|Vector|Lerp(Vector) (Variables|Default|GetBaseLocation) (Variables|Default|GetEndLocation) _newtrack_0) false false))))

(event EventBeginPlay
  (Variables|Default|SetBaseLocation (Transformation|GetWorldLocation (Variables|Default|GetDoor)))
  (Variables|Default|SetEndLocation (Math|Vector|MakeVector (+ (.x (Variables|Default|GetBaseLocation)) (Variables|Default|GetMoveXValue)) (+ (.y (Variables|Default|GetBaseLocation)) (Variables|Default|GetMoveYValue)) (+ (.z (Variables|Default|GetBaseLocation)) (Variables|Default|GetMoveZValue)))))

(fn ConstructionScript)