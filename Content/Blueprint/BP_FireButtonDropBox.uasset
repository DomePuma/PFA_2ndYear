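; Fire-character pressure plate that drops a portable puzzle box from a drop tube when BP_FireCharacter_2 hits it.
; The first hit always spawns, later hits only if CanSpawnAgain is set, and a delayed SpawnTrigger reset enforces a cooldown between drops.
; Activation plays plate and tube sounds, then spawns the BoxType variant (pressure plate, platform or big) at DropPoint, passing on Zone and enabling physics.
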(event Custom|Cooldown
  (Variables|Default|SetSpawnTrigger false)
  (Utilities|FlowControl|Delay (Variables|Default|GetSpawnCooldown))
  (Variables|Default|SetSpawnTrigger true))

(event Custom|ActivateInterction
  (bind _droppoint (Variables|Default|GetDropPoint))
  (bind _returnvalue (Transformation|GetWorldTransform _droppoint))
  (Audio|PlaySoundatLocation "/Game/Audio/Sounds/pressure_plate_pressed.pressure_plate_pressed" (Transformation|GetWorldLocation (Variables|Default|GetPressurePlate)) "0, 0, 0" 1.0 1.0 0.0 0 0 0 0)
  (Audio|PlaySoundatLocation "/Game/Audio/Sounds/Boxspawner_opening.Boxspawner_opening" (Transformation|GetWorldLocation (Variables|Default|GetDropTube)) "0, 0, 0" 1.0 1.0 0.0 0 0 0 0)
  (switch Utilities|FlowControl|Switch|SwitchonE_BoxType (Variables|Default|GetBoxType)
    (:NewEnumerator0
      (bind _returnvalue_2 (Game|SpawnActorfromClass "/Game/Blueprint/BP_PortablePressurePlateBox.BP_PortablePressurePlateBox_C" (Math|Transform|MakeTransform (.location _returnvalue) (.rotation _returnvalue) "1.000000,1.000000,1.000000") "Undefined" 0 0))
      (Variables|/Game/Blueprint/BP_PortablePressurePlateBox.BP_PortablePressurePlateBox_C|SetZone _returnvalue_2 (Variables|Default|GetZone))
      (Physics|SetSimulatePhysics (Variables|/Game/Blueprint/BP_InteractableObject.BP_InteractableObject_C|GetCube _returnvalue_2) true))
    (:NewEnumerator1
      (bind _returnvalue_3 (Game|SpawnActorfromClass "/Game/Blueprint/BP_PortablePlatformBox.BP_PortablePlatformBox_C" (Math|Transform|MakeTransform (.location _returnvalue) (.rotation _returnvalue) "1.000000,1.000000,1.000000") "Undefined" 0 0))
      (Variables|/Game/Blueprint/BP_PortablePlatformBox.BP_PortablePlatformBox_C|SetZone _returnvalue_3 (Variables|Default|GetZone))
      (Physics|SetSimulatePhysics (Variables|/Game/Blueprint/BP_InteractableObject.BP_InteractableObject_C|GetCube _returnvalue_3) true))
    (:NewEnumerator2
      (bind _returnvalue_4 (Game|SpawnActorfromClass "/Game/Blueprint/BP_PortableBigBox.BP_PortableBigBox_C" (Math|Transform|MakeTransform (.location _returnvalue) (.rotation _returnvalue) "1.000000,1.000000,1.000000") "Undefined" 0 0))
      (Variables|/Game/Blueprint/BP_PortableBigBox.BP_PortableBigBox_C|SetZone _returnvalue_4 (Variables|Default|GetZone))
      (Physics|SetSimulatePhysics (Variables|/Game/Blueprint/BP_InteractableObject.BP_InteractableObject_C|GetCube _returnvalue_4) true))))

(event Collision|EventHit
  (params (MyComp :type Primitive%20Component%20Object%20Reference) (Other :type Actor%20Object%20Reference) (OtherComp :type Primitive%20Component%20Object%20Reference) (bSelfMoved :type Boolean) (HitLocation :type Vector :default "0, 0, 0") (HitNormal :type Vector :default "0, 0, 0") (NormalImpulse :type Vector :default "0, 0, 0") (Hit :type Hit%20Result%20Structure%20%28by%20ref%29))
  (bind _cubespawncounter (Variables|Default|GetCubeSpawnCounter))
  (if (Variables|Default|GetSpawnTrigger)
    (Utilities|Casting|CastToBP_FireCharacter_2 Other)
    (if (<= _cubespawncounter 0)
      (CallFunction|ActivateInterction :!label _label)
      (Math|Integer|IncrementInt _cubespawncounter
        (:%20%20
          (CallFunction|Cooldown)))
      (elif (Variables|Default|GetCanSpawnAgain)
        (goto _label)))))

(fn ConstructionScript)