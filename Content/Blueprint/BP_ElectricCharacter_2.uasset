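; Playable electric character that operates interactable objects and sprints on a limited gauge.
; Interact, when grounded, casts the first overlapping object to activate button-driven doors, platforms or drop boxes, or trigger an incubator level change.
; Releasing or leaving the interaction box deactivates the stored object, closing hold-button doors.
; Tick zeroes control rotation, eases airborne velocity toward a cap, and drives sprint speed, effects and gauge recharge.
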(event OnComponentEndOverlap(InteractionBox)
  (params (OverlappedComponent :type Primitive%20Component%20Object%20Reference) (OtherActor :type Actor%20Object%20Reference) (OtherComp :type Primitive%20Component%20Object%20Reference) (OtherBodyIndex :type Integer))
  (Variables|Default|SetIsInInteraction false)
  (bind _asbp_interactable_object (Utilities|Casting|CastToBP_InteractableObject (Variables|Default|GetInteractableObjectRef)))
  (Default|DesactivateInteraction _asbp_interactable_object)
  (switch Utilities|FlowControl|Switch|SwitchonE_InteractableButtonType (Variables|/Game/Blueprint/BP_InteractableObject.BP_InteractableObject_C|GetObjectType _asbp_interactable_object)
    (:NewEnumerator1
      (bind _asbp_hold_button_door (Utilities|Casting|CastToBP_HoldButtonDoor _asbp_interactable_object))
      (Default|CloseDoor _asbp_hold_button_door)
      (Variables|Default|SetInteractableObjectRef 0))))

(event EventBeginPlay
  (Variables|Default|SetBaseSpeed (Class|MovementComponent|GetMaxSpeed (Variables|Character|GetCharacterMovement))))

(event EventTick
  (params (DeltaSeconds :type Float%20%28single-precision%29))
  (CallFunction|SetRotationController)
  (CallFunction|SetAirVelocity DeltaSeconds)
  (CallFunction|Sprint)
  (if (<= (.z (Variables|/Script/Engine.MovementComponent|GetVelocity (Variables|Character|GetCharacterMovement))) 0.0)
    (Variables|Default|SetIsInteracting false)))

(event Input|ActionEvents|InputActionInteractElectric
  (params (Key :type Key%20Structure :default "None"))
  (bind _interactionbox (Variables|Default|GetInteractionBox))
  (bind _overlappingactors (Collision|GetOverlappingActors _interactionbox "/Game/Blueprint/BP_InteractableObject.BP_InteractableObject_C" :!class /Script/Engine.PrimitiveComponent))
  (bind _output (Utilities|Array|Get(acopy) _overlappingactors))
  (bind _returnvalue (Collision|IsOverlappingActor _interactionbox _output :!class /Script/Engine.PrimitiveComponent))
  (:Pressed
    (if (not (AI|Components|NavMovement|IsFalling (Variables|Character|GetCharacterMovement)))
      (if _returnvalue
        (Variables|Default|SetInteractableObjectRef _output)
        (bind _asbp_interactable_object (Utilities|Casting|CastToBP_InteractableObject _output))
        (switch Utilities|FlowControl|Switch|SwitchonE_InteractableButtonType (Variables|/Game/Blueprint/BP_InteractableObject.BP_InteractableObject_C|GetObjectType _asbp_interactable_object)
          (:NewEnumerator1
            (bind _asbp_hold_button_door (Utilities|Casting|CastToBP_HoldButtonDoor _asbp_interactable_object)
              (:then
                (Default|ActivateInteraction _asbp_hold_button_door)
                (Default|OpenDoor _asbp_hold_button_door)
                (Variables|Default|SetIsInInteraction true)
                (Utilities|FlowControl|Delay 0.2)
                (Variables|Default|SetIsInteracting false))
              (:CastFailed
                (bind _asbp_simple_button_door (Utilities|Casting|CastToBP_SimpleButtonDoor _asbp_interactable_object)
                  (:then
                    (Default|ActivateInteraction _asbp_simple_button_door)
                    (Variables|Default|SetIsInInteraction true)
                    (Utilities|FlowControl|Delay 0.2)
                    (Variables|Default|SetIsInteracting false))
                  (:CastFailed
                    (bind _asbp_simple_button_platform (Utilities|Casting|CastToBP_SimpleButtonPlatform _asbp_interactable_object)
                      (:then
                        (Default|ActivateInteraction _asbp_simple_button_platform)
                        (Variables|Default|SetIsInInteraction true)
                        (Utilities|FlowControl|Delay 0.2)
                        (Variables|Default|SetIsInteracting false))
                      (:CastFailed
                        (bind _asbp_electric_button_drop_box (Utilities|Casting|CastToBP_ElectricButtonDropBox _asbp_interactable_object))
                        (Default|ActivateInteraction _asbp_electric_button_drop_box)
                        (Variables|Default|SetIsInInteraction true)
                        (Utilities|FlowControl|Delay 0.2)
                        (Variables|Default|SetIsInteracting false))))))))
          (:NewEnumerator5
            (bind _asbp_incubator (Utilities|Casting|CastToBP_Incubator _asbp_interactable_object))
            (Default|ChangeLevel _asbp_incubator))))))
  (:Released
    (if _returnvalue
      (Variables|Default|SetIsInInteraction false)
      (bind _asbp_interactable_object_2 (Utilities|Casting|CastToBP_InteractableObject (Variables|Default|GetInteractableObjectRef)))
      (Default|DesactivateInteraction _asbp_interactable_object_2)
      (switch Utilities|FlowControl|Switch|SwitchonE_InteractableButtonType (Variables|/Game/Blueprint/BP_InteractableObject.BP_InteractableObject_C|GetObjectType _asbp_interactable_object_2)
        (:NewEnumerator1
          (bind _asbp_hold_button_door_2 (Utilities|Casting|CastToBP_HoldButtonDoor _asbp_interactable_object_2))
          (Default|CloseDoor _asbp_hold_button_door_2)
          (Variables|Default|SetInteractableObjectRef 0)))
      (else
        (Variables|Default|SetIsInInteraction false)))))

(event Input|ActionEvents|InputActionSprint/FireBall
  (params (Key :type Key%20Structure :default "None"))
  (:Pressed
    (Variables|Default|SetIsRunning true))
  (:Released
    (Variables|Default|SetIsRunning false)))

(fn ConstructionScript
  (|CallParentFunction))

(fn SetRotationController
  (Pawn|SetControlRotation (Pawn|GetController) (Math|Rotator|MakeRotator 0.0 0.0 0.0)))

(fn SetAirVelocity
  (params (DeltaTime :type Float%20%28single-precision%29))
  (bind _charactermovement (Variables|Character|GetCharacterMovement))
  (bind _maxairspeed (Variables|Default|GetMaxAirSpeed))
  (if (AI|Components|NavMovement|IsFalling _charactermovement)
    (if (> (Math|Vector|VectorLength (Variables|/Script/Engine.MovementComponent|GetVelocity _charactermovement)) _maxairspeed)
      (Variables|/Script/Engine.MovementComponent|SetVelocity _charactermovement (Math|Interpolation|VInterpTo (Variables|/Script/Engine.MovementComponent|GetVelocity _charactermovement) (* (/ _maxairspeed (Math|Vector|VectorLength (Variables|/Script/Engine.MovementComponent|GetVelocity _charactermovement))) (Variables|/Script/Engine.MovementComponent|GetVelocity _charactermovement)) DeltaTime 0.0)))))

(fn Sprint
  (bind _yomasprint (Variables|Default|GetYomaSprint))
  (bind _charactermovement (Variables|Character|GetCharacterMovement))
  (bind _yomasprint1 (Variables|Default|GetYomaSprint1))
  (if (and (Variables|Default|GetIsRunning) (> (Variables|Default|GetSprintGauge) 0.0))
    (Components|Activation|Activate _yomasprint1 false)
    (Components|Activation|Activate _yomasprint false)
    (Variables|Default|SetSprintGauge (- (Variables|Default|GetSprintGauge) (Utilities|Time|GetWorldDeltaSeconds)))
    (Variables|/Script/Engine.CharacterMovementComponent|SetMaxWalkSpeed _charactermovement (Variables|Default|GetSprintSpeed))
    (else
      (Components|Activation|Deactivate _yomasprint1)
      (Components|Activation|Deactivate _yomasprint)
      (Variables|Default|SetIsRunning false)
      (Variables|/Script/Engine.CharacterMovementComponent|SetMaxWalkSpeed _charactermovement (Variables|Default|GetBaseSpeed))
      (CallFunction|ReloadSpeedGauge))))

(fn ReloadSpeedGauge
  (if (and (not (Variables|Default|GetIsRunning)) (< (Variables|Default|GetSprintGauge) (Variables|Default|GetSprintTime)))
    (Variables|Default|SetSprintGauge (+ (Variables|Default|GetSprintGauge) (Utilities|Time|GetWorldDeltaSeconds)))))