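; Box-triggered button that drops a new portable box when a pressure plate box overlaps its trigger.
; The overlap activates the incoming box if it cannot be repicked, then spawns a pressure plate, platform or big box, chosen by BoxType, at DropPoint with physics enabled.
; A spawn counter limits this to one drop unless CanSpawnAgain allows repeats.
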(event OnComponentBeginOverlap(Box)
  (params (OverlappedComponent :type Primitive%20Component%20Object%20Reference) (OtherActor :type Actor%20Object%20Reference) (OtherComp :type Primitive%20Component%20Object%20Reference) (OtherBodyIndex :type Integer) (bFromSweep :type Boolean) (SweepResult :type Hit%20Result%20Structure%20%28by%20ref%29))
  (bind _cubespawncounter (Variables|Default|GetCubeSpawnCounter))
  (bind _asbp_portable_pressure_plate_box (Utilities|Casting|CastToBP_PortablePressurePlateBox OtherActor))
  (if (<= _cubespawncounter 0)
    (if (Variables|/Game/Blueprint/BP_PortablePressurePlateBox.BP_PortablePressurePlateBox_C|GetCanBeRepicked _asbp_portable_pressure_plate_box) :!label _label
      _
      (else
        (Default|ActivateInteraction _asbp_portable_pressure_plate_box)))
    (CallFunction|ActivateInterction)
    (Math|Integer|IncrementInt _cubespawncounter)
    (elif (Variables|Default|GetCanSpawnAgain)
      (goto _label))))

(event Custom|ActivateInterction
  (bind _droppoint (Variables|Default|GetDropPoint))
  (bind _returnvalue (Transformation|GetWorldTransform _droppoint))
  (switch Utilities|FlowControl|Switch|SwitchonE_BoxType (Variables|Default|GetBoxType)
    (:NewEnumerator0
      (bind _returnvalue_2 (Game|SpawnActorfromClass "/Game/Blueprint/BP_PortablePressurePlateBox.BP_PortablePressurePlateBox_C" (Math|Transform|MakeTransform (.location _returnvalue) (.rotation _returnvalue) "1.000000,1.000000,1.000000") "Undefined" 0 0))
      (Physics|SetSimulatePhysics (Variables|/Game/Blueprint/BP_InteractableObject.BP_InteractableObject_C|GetCube _returnvalue_2) true))
    (:NewEnumerator1
      (bind _returnvalue_3 (Game|SpawnActorfromClass "/Game/Blueprint/BP_PortablePlatformBox.BP_PortablePlatformBox_C" (Math|Transform|MakeTransform (.location _returnvalue) (.rotation _returnvalue) "1.000000,1.000000,1.000000") "Undefined" 0 0))
      (Physics|SetSimulatePhysics (Variables|/Game/Blueprint/BP_InteractableObject.BP_InteractableObject_C|GetCube _returnvalue_3) true))
    (:NewEnumerator2
      (bind _returnvalue_4 (Game|SpawnActorfromClass "/Game/Blueprint/BP_PortableBigBox.BP_PortableBigBox_C" (Math|Transform|MakeTransform (.location _returnvalue) (.rotation _returnvalue) "1.000000,1.000000,1.000000") "Undefined" 0 0))
      (Physics|SetSimulatePhysics (Variables|/Game/Blueprint/BP_InteractableObject.BP_InteractableObject_C|GetCube _returnvalue_4) true))))

(fn ConstructionScript)