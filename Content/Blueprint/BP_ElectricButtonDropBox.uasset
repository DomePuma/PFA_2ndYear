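; Interactable button that drops a portable pressure plate, platform or big box from a drop point, chosen by BoxType.
; Interaction plays button and opening sounds, spawns the box with physics and passes it the Zone.
; The first spawn is always allowed, later ones require CanSpawnAgain, and a SpawnTrigger cooldown spaces them out.
; A sphere overlap shows the prompt widget to BP_ElectricCharacter_2 only when CanSpawnAgain is set.
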(event OnComponentBeginOverlap(Sphere)
  (params (OverlappedComponent :type Primitive%20Component%20Object%20Reference) (OtherActor :type Actor%20Object%20Reference) (OtherComp :type Primitive%20Component%20Object%20Reference) (OtherBodyIndex :type Integer) (bFromSweep :type Boolean) (SweepResult :type Hit%20Result%20Structure%20%28by%20ref%29))
  ;[1 1 1] Interact_prompt
  (Utilities|Casting|CastToBP_ElectricCharacter_2 OtherActor)
  (if (Variables|Default|GetCanSpawnAgain)
    (Rendering|SetVisibility (Variables|Default|GetWidget) true false)))

(event OnComponentEndOverlap(Sphere)
  (params (OverlappedComponent :type Primitive%20Component%20Object%20Reference) (OtherActor :type Actor%20Object%20Reference) (OtherComp :type Primitive%20Component%20Object%20Reference) (OtherBodyIndex :type Integer))
  ;[1 1 1] Interact_prompt
  (Utilities|Casting|CastToBP_ElectricCharacter_2 OtherActor)
  (Rendering|SetVisibility (Variables|Default|GetWidget) false false))

(event Custom|Cooldown
  (Variables|Default|SetSpawnTrigger false)
  (Utilities|FlowControl|Delay (Variables|Default|GetSpawnCooldown))
  (Variables|Default|SetSpawnTrigger true))

(event Custom|ActivateInterction
  (bind _droppoint (Variables|Default|GetDropPoint))
  (bind _returnvalue (Transformation|GetWorldTransform _droppoint))
  (Audio|PlaySoundatLocation "/Game/Audio/Sounds/générator_activation.générator_activation" (Transformation|GetWorldLocation (Variables|Default|GetButton)) "0, 0, 0" 1.0 1.0 0.0 0 0 0 0)
  (Audio|PlaySoundatLocation "/Game/Audio/Sounds/Boxspawner_opening.Boxspawner_opening" (Transformation|GetWorldLocation (Variables|Default|GetDropPoint)) "0, 0, 0" 1.0 1.0 0.0 0 0 0 0)
  (switch Utilities|FlowControl|Switch|SwitchonE_BoxType (Variables|Default|GetBoxType)
    (:NewEnumerator0
      (bind _returnvalue_2 (Game|SpawnActorfromClass "/Game/Blueprint/BP_PortablePressurePlateBox.BP_PortablePressurePlateBox_C" (Math|Transform|MakeTransform (.location _returnvalue) "0, 0, 0" "1.000000,1.000000,1.000000") "Undefined" 0 0))
      (Variables|/Game/Blueprint/BP_PortablePressurePlateBox.BP_PortablePressurePlateBox_C|SetZone _returnvalue_2 (Variables|Default|GetZone))
      (Physics|SetSimulatePhysics (Variables|/Game/Blueprint/BP_InteractableObject.BP_InteractableObject_C|GetCube _returnvalue_2) true))
    (:NewEnumerator1
      (bind _returnvalue_3 (Game|SpawnActorfromClass "/Game/Blueprint/BP_PortablePlatformBox.BP_PortablePlatformBox_C" (Math|Transform|MakeTransform (.location _returnvalue) "0, 0, 0" "1.000000,1.000000,1.000000") "Undefined" 0 0))
      (Variables|/Game/Blueprint/BP_PortablePlatformBox.BP_PortablePlatformBox_C|SetZone _returnvalue_3 (Variables|Default|GetZone))
      (Physics|SetSimulatePhysics (Variables|/Game/Blueprint/BP_InteractableObject.BP_InteractableObject_C|GetCube _returnvalue_3) true))
    (:NewEnumerator2
      (bind _returnvalue_4 (Game|SpawnActorfromClass "/Game/Blueprint/BP_PortableBigBox.BP_PortableBigBox_C" (Math|Transform|MakeTransform (.location _returnvalue) "0, 0, 0" "1.000000,1.000000,1.000000") "Undefined" 0 0))
      (Variables|/Game/Blueprint/BP_PortableBigBox.BP_PortableBigBox_C|SetZone _returnvalue_4 (Variables|Default|GetZone))
      (Physics|SetSimulatePhysics (Variables|/Game/Blueprint/BP_InteractableObject.BP_InteractableObject_C|GetCube _returnvalue_4) true))))

(event EventBeginPlay
  ;[1 1 1] Interact_prompt
  (Rendering|SetVisibility (Variables|Default|GetWidget) false false))

(event EventActivateInteraction
  (bind _cubespawncounter (Variables|Default|GetCubeSpawnCounter))
  (if (Variables|Default|GetSpawnTrigger)
    (if (<= _cubespawncounter 0)
      (CallFunction|ActivateInterction :!label _label)
      (Math|Integer|IncrementInt _cubespawncounter
        (:%20%20
          (CallFunction|Cooldown)))
      (elif (Variables|Default|GetCanSpawnAgain)
        (goto _label)))))

(fn ConstructionScript)