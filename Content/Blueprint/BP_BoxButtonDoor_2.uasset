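; Pressure plate and door actor that opens when a BP_PortablePressurePlateBox overlaps its trigger Box.
; On overlap it triggers the box's own interaction if that box cannot be repicked, then plays plate and door sounds.
; A timeline lerps the door from its current location toward its BeginPlay location plus configurable XYZ offsets.
; No closing logic exists.
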(event OnComponentBeginOverlap(Box)
  (params (OverlappedComponent :type Primitive%20Component%20Object%20Reference) (OtherActor :type Actor%20Object%20Reference) (OtherComp :type Primitive%20Component%20Object%20Reference) (OtherBodyIndex :type Integer) (bFromSweep :type Boolean) (SweepResult :type Hit%20Result%20Structure%20%28by%20ref%29))
  (bind _asbp_portable_pressure_plate_box (Utilities|Casting|CastToBP_PortablePressurePlateBox OtherActor))
  (if (Variables|/Game/Blueprint/BP_PortablePressurePlateBox.BP_PortablePressurePlateBox_C|GetCanBeRepicked _asbp_portable_pressure_plate_box)
    _
    (else
      (Default|ActivateInteraction _asbp_portable_pressure_plate_box)))
  (CallFunction|ActivateInteraction))

(event Custom|ActivateInteraction
  (bind _baselocation (Variables|Default|GetBaseLocation))
  (Audio|PlaySoundatLocation "/Game/Audio/Sounds/pressure_plate_pressed.pressure_plate_pressed" (Transformation|GetWorldLocation (Variables|Default|GetPressurePlate)) "0, 0, 0" 1.0 1.0 0.0 0 0 0 0)
  (Audio|PlaySoundatLocation "/Game/Audio/Sounds/Door_opening.Door_opening" (Transformation|GetWorldLocation (Variables|Default|GetDoor)) "0, 0, 0" 1.0 1.0 0.0 0 0 0 0)
  (bind _newtrack_0 (Timeline|OpenDoor Play)
    (:Update
      (Transformation|SetWorldLocation (Variables|Default|GetDoor) (Math|Vector|Lerp(Vector) (Transformation|GetWorldLocation (Variables|Default|GetDoor)) (Math|Vector|MakeVector (+ (.x _baselocation) (Variables|Default|GetMoveXValue)) (+ (.y _baselocation) (Variables|Default|GetMoveYValue)) (+ (.z _baselocation) (Variables|Default|GetMoveZValue))) _newtrack_0) false false))))

(event EventBeginPlay
  (Variables|Default|SetBaseLocation (Transformation|GetWorldLocation (Variables|Default|GetDoor))))

(fn ConstructionScript)