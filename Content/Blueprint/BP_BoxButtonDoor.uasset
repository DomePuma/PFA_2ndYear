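; BP_BoxButtonDoor is a door with a button that opens it when a BP_PortablePressurePlateBox overlaps the button.
; BeginPlay stores the door's starting location, and the overlap triggers ActivateInteraction, which plays the OpenDoor timeline.
; Each update lerps the door from its current location toward that start plus configurable X, Y and Z offsets.
; No logic closes the door again.
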(event OnComponentBeginOverlap(Button)
  (params (OverlappedComponent :type Primitive%20Component%20Object%20Reference) (OtherActor :type Actor%20Object%20Reference) (OtherComp :type Primitive%20Component%20Object%20Reference) (OtherBodyIndex :type Integer) (bFromSweep :type Boolean) (SweepResult :type Hit%20Result%20Structure%20%28by%20ref%29))
  (Utilities|Casting|CastToBP_PortablePressurePlateBox OtherActor)
  (CallFunction|ActivateInteraction))

(event Custom|ActivateInteraction
  (bind _baselocation (Variables|Default|GetBaseLocation))
  (bind _newtrack_0 (Timeline|OpenDoor Play)
    (:Update
      (Transformation|SetWorldLocation (Variables|Default|GetDoor) (Math|Vector|Lerp(Vector) (Transformation|GetWorldLocation (Variables|Default|GetDoor)) (Math|Vector|MakeVector (+ (.x _baselocation) (Variables|Default|GetMoveXValue)) (+ (.y _baselocation) (Variables|Default|GetMoveYValue)) (+ (.z _baselocation) (Variables|Default|GetMoveZValue))) _newtrack_0) false false))))

(event EventBeginPlay
  (Variables|Default|SetBaseLocation (Transformation|GetWorldLocation (Variables|Default|GetDoor))))

(fn ConstructionScript)